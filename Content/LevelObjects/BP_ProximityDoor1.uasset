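; A proximity door that slides open when an in-game character enters its trigger box and closes once the box is empty.
; Overlap events adjust NumOpenDoor for any other actor, but only characters call OpenDoor or CloseDoor.
; OpenDoor plays a timeline that moves the mesh, and CloseDoor reverses it when the count reaches zero.
; Server checks and OnRep functions are empty, and debug prints remain.
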(event OnComponentEndOverlap(Box)
  (params (OverlappedComponent :type Primitive%20Component%20Object%20Reference) (OtherActor :type Actor%20Object%20Reference) (OtherComp :type Primitive%20Component%20Object%20Reference) (OtherBodyIndex :type Integer))
  ;[1 1 1] THIS IS MESSY BUT I DONT WANT TO TOUCH IT CAUSE IT WORKS
  (if (== OtherActor self)
    _
    (else
      (if (Networking|IsServer)
        _
        (else
          _))
      (Variables|Default|SetnumOpenDoor (+ (Variables|Default|GetnumOpenDoor) -1))))
  (Utilities|Casting|CastToBP_InGame_Character OtherActor)
  (CallFunction|CloseDoor))

(event OnComponentBeginOverlap(Box)
  (params (OverlappedComponent :type Primitive%20Component%20Object%20Reference) (OtherActor :type Actor%20Object%20Reference) (OtherComp :type Primitive%20Component%20Object%20Reference) (OtherBodyIndex :type Integer) (bFromSweep :type Boolean) (SweepResult :type Hit%20Result%20Structure%20%28by%20ref%29))
  ;[1 1 1] THIS IS MESSY BUT I DONT WANT TO TOUCH IT CAUSE IT WORKS
  (if (== OtherActor self)
    _
    (else
      (if (Networking|IsServer)
        _
        (else
          _))
      (Variables|Default|SetnumOpenDoor (+ (Variables|Default|GetnumOpenDoor) 1))))
  (Utilities|Casting|CastToBP_InGame_Character OtherActor)
  (CallFunction|OpenDoor))

(event Custom|Close%20Door
  (bind _numopendoor (Variables|Default|GetnumOpenDoor))
  ;[1 1 1] THIS IS MESSY BUT I DONT WANT TO TOUCH IT CAUSE IT WORKS
  (Development|PrintString (Utilities|String|ToString(Integer) _numopendoor))
  (if (== _numopendoor 0)
    (Development|PrintString "REVERSE")
    (bind _door_sliding (Timeline|Door%20Animation Reverse)
      (:Update
        (Transformation|SetRelativeLocation (Variables|Default|GetDoorMesh) _door_sliding false false)))))

(event Custom|Open%20Door
  ;[1 1 1] THIS IS MESSY BUT I DONT WANT TO TOUCH IT CAUSE IT WORKS
  (Development|PrintString (Utilities|String|ToString(Integer) (Variables|Default|GetnumOpenDoor)))
  (Development|PrintString "OPEN")
  (Utilities|Casting|CastToBP_InGame_Character (Game|GetPlayerCharacter 0))
  (bind _door_sliding (Timeline|Door%20Animation Play)
    (:Update
      (Transformation|SetRelativeLocation (Variables|Default|GetDoorMesh) _door_sliding false false))))

(fn ConstructionScript)

(fn OnRepDontCloseDoor)

(fn OnRepNumOpenDoor)