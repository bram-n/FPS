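; Health pickup actor that heals the player character on touch.
; When its Box component begins overlapping a BP_InGame_Character, it adds a fixed amount directly to that character's Health, capped at 100.
; It then prints the new health to the screen and destroys itself, even if the character was already at full health.
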(event OnComponentBeginOverlap(Box)
  (params (OverlappedComponent :type Primitive%20Component%20Object%20Reference) (OtherActor :type Actor%20Object%20Reference) (OtherComp :type Primitive%20Component%20Object%20Reference) (OtherBodyIndex :type Integer) (bFromSweep :type Boolean) (SweepResult :type Hit%20Result%20Structure%20%28by%20ref%29))
  (bind _asbp_in_game_character (Utilities|Casting|CastToBP_InGame_Character OtherActor))
  (if (> (Variables|/Game/Framework/BP_InGame_Character.BP_InGame_Character_C|GetHealth _asbp_in_game_character) 75.0)
    (Variables|/Game/Framework/BP_InGame_Character.BP_InGame_Character_C|SetHealth _asbp_in_game_character 1e+02)
    (else
      (Variables|/Game/Framework/BP_InGame_Character.BP_InGame_Character_C|SetHealth _asbp_in_game_character (+ (Variables|/Game/Framework/BP_InGame_Character.BP_InGame_Character_C|GetHealth _asbp_in_game_character) 25.0))))
  (Development|PrintString (Utilities|String|Append "Health: " (Utilities|String|ToString(Float) (Variables|/Game/Framework/BP_InGame_Character.BP_InGame_Character_C|GetHealth _asbp_in_game_character))))
  (Actor|DestroyActor))

(event EventBeginPlay)

(event Collision|EventActorBeginOverlap
  (params (OtherActor :type Actor%20Object%20Reference)))

(event EventTick
  (params (DeltaSeconds :type Float%20%28single-precision%29)))

(fn ConstructionScript)