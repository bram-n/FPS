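; BP_InGame_Gamemode2 is an in-game game mode that splits joining players into two teams and runs a pre-match countdown.
; PostLogin records each player controller, using a FlipFlop to alternate team arrays and set CurrentTeam on the player state, while counting controllers.
; A looping one-second timer counts down while exactly two controllers are counted, then clears itself and calls StartMatch, which is still empty.
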(event Custom|GetReady%20Timer%20Event
  (if (== (Variables|Default|GetTotalControllers) 2)
    (bind _result (Math|Integer|DecrementInt (Variables|Default|GetGetReadyTimerInteger))
      (:%20%20
        (Development|PrintString (Utilities|String|Append "Game Begins in:" (Utilities|String|ToString(Integer) _result)))
        (if (<= _result 0)
          (Utilities|Time|ClearandInvalidateTimerbyHandle (Variables|Default|GetGetReadyTimerHandle))
          (CallFunction|StartMatch))))))

(event Custom|Start%20Match)

(event EventBeginPlay
  (bind _returnvalue (Utilities|Time|SetTimerbyEvent (delegate Custom|GetReady%20Timer%20Event) 1.0 true))
  (Variables|Default|SetGetReadyTimerHandle _returnvalue))

(event EventPostLogin
  (params (NewPlayer :type Player%20Controller%20Object%20Reference))
  (bind _asbp_in_game_player_controller (Utilities|Casting|CastToBP_InGame_PlayerController NewPlayer))
  (bind _playerstate (Variables|/Script/Engine.Controller|GetPlayerState _asbp_in_game_player_controller))
  (bind _asbp_in_game_player_controller_2 (Utilities|Casting|CastToBP_InGame_PlayerController NewPlayer))
  (Utilities|Array|Add (Variables|Default|GetAllConnectedPlayers) _asbp_in_game_player_controller_2)
  (Utilities|FlowControl|FlipFlop
    (:A
      (Utilities|Array|Add (Variables|Default|GetTeam1Controllers) _asbp_in_game_player_controller)
      (bind _asbp_in_game_player_state (Utilities|Casting|CastToBP_InGame_PlayerState _playerstate))
      (Variables|/Game/Framework/BP_InGame_PlayerState.BP_InGame_PlayerState_C|SetCurrent%20Team _asbp_in_game_player_state "NewEnumerator0"))
    (:B
      (Utilities|Array|Add (Variables|Default|GetTeam2Controllers) _asbp_in_game_player_controller)
      (bind _asbp_in_game_player_state_2 (Utilities|Casting|CastToBP_InGame_PlayerState _playerstate))
      (Variables|/Game/Framework/BP_InGame_PlayerState.BP_InGame_PlayerState_C|SetCurrent%20Team _asbp_in_game_player_state_2 "NewEnumerator1")))
  (bind _output_get (Variables|Default|SetTotalControllers (+ (Variables|Default|GetTotalControllers) 1)))
  (Development|PrintString (Utilities|String|Append "Total Controllers: " (Utilities|String|ToString(Integer) _output_get))))

(fn ConstructionScript)