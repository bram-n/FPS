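; BP_Menu_Gamemode is the menu game mode that tracks players in the multiplayer lobby.
; New players entering the L Lobby level are added to a controller list, and their controllers create the lobby menu and run initial setup.
; Logout removes the player and triggers UpdateLobby, which rebuilds the profile list and pushes it to every remaining controller to update player names.
; Joining does not call UpdateLobby here.
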(event Custom|UpdateLobby
  (params (PlayerNames :type Boolean))
  (if PlayerNames
    (Utilities|Array|Clear (Variables|Default|GetAllPlayerProfiles))
    (for _array_element (Variables|Default|GetAllConnectedPlayers)
      (Utilities|Array|Add (Variables|Default|GetAllPlayerProfiles) (Variables|/Game/Framework/BP_Menu_PlayerController.BP_Menu_PlayerController_C|GetPlayer%20Profile _array_element)))
    (for _array_element_2 (Variables|Default|GetAllConnectedPlayers)
      (if PlayerNames
        (Default|UpdatePlayerNames _array_element_2 (Variables|Default|GetAllPlayerProfiles))))))

(event EventBeginPlay)

(event EventTick
  (params (DeltaSeconds :type Float%20%28single-precision%29)))

(event EventHandleStartingNewPlayer
  (params (NewPlayer :type Player%20Controller%20Object%20Reference))
  (Development|PrintString "Entering new level...")
  (bind _returnvalue (Game|GetCurrentLevelName true))
  (switch string _returnvalue
    (:L_Lobby
      (bind _asbp_menu_player_controller (Utilities|Casting|CastToBP_Menu_PlayerController NewPlayer))
      (Utilities|Array|Add (Variables|Default|GetAllConnectedPlayers) _asbp_menu_player_controller)
      (Default|CreateLobbyMenu _asbp_menu_player_controller)
      (Default|InitialSetup _asbp_menu_player_controller))))

(event EventOnLogout
  (params (ExitingController :type Controller%20Object%20Reference))
  (bind _asbp_menu_player_controller (Utilities|Casting|CastToBP_Menu_PlayerController ExitingController))
  (Utilities|Array|RemoveItem (Variables|Default|GetAllConnectedPlayers) _asbp_menu_player_controller)
  (CallFunction|UpdateLobby true))

(fn ConstructionScript)