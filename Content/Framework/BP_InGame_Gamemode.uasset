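; BP_InGame_Gamemode is the in-game GameMode that tracks connected players and spawns their team characters.
; PostLogin adds each joining BP_InGame_PlayerController to AllConnectedPlayers.
; SpawnPlayer spawns a BP_InGame_Character at a random PlayerStart tagged with the team, then after a short delay possesses it with the given controller and sets its TeamTag.
; BeginPlay and StartMatch are empty, and nothing in this graph calls SpawnPlayer.
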(event Custom|SpawnPlayer
  (params (TeamTag :type Name) (PlayerController :type Player%20Controller%20Object%20Reference))
  (bind _outactors (Actor|GetAllActorsOfClasswithTag "/Script/Engine.PlayerStart" TeamTag))
  (bind _returnvalue (Game|SpawnActorfromClass "/Game/Framework/BP_InGame_Character.BP_InGame_Character_C" (Transformation|GetActorTransform (.OutItem (Utilities|Array|Random _outactors))) "Undefined" "MultiplyWithRoot" 0 0))
  (Utilities|FlowControl|Delay 0.2)
  (Pawn|Possess PlayerController _returnvalue)
  (Variables|/Game/Framework/BP_InGame_Character.BP_InGame_Character_C|SetTeamTag _returnvalue TeamTag))

(event Custom|Start%20Match)

(event EventBeginPlay)

(event EventPostLogin
  (params (NewPlayer :type Player%20Controller%20Object%20Reference))
  (bind _asbp_in_game_player_controller (Utilities|Casting|CastToBP_InGame_PlayerController NewPlayer))
  (Utilities|Array|Add (Variables|Default|GetAllConnectedPlayers) _asbp_in_game_player_controller))

(fn ConstructionScript)