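; Capture-the-flag base actor that tracks whether its flag is home and holds the owning team's points.
; A sphere trigger, sized in the construction script, checks each overlapping character's team tag.
; Enemies take the flag if it is present, while returning carriers score a point and restore the enemy base's flag.
; Server-named events update that state, and ChangeState swaps the enemy base's flag mesh to show it.
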(event OnComponentBeginOverlap(Radious)
  (params (OverlappedComponent :type Primitive%20Component%20Object%20Reference) (OtherActor :type Actor%20Object%20Reference) (OtherComp :type Primitive%20Component%20Object%20Reference) (OtherBodyIndex :type Integer) (bFromSweep :type Boolean) (SweepResult :type Hit%20Result%20Structure%20%28by%20ref%29))
  (bind _asbp_in_game_character (Utilities|Casting|CastToBP_InGame_Character OtherActor))
  (if (== (Variables|/Game/Framework/BP_InGame_Character.BP_InGame_Character_C|GetTeamTag _asbp_in_game_character) (Variables|Default|GetOwnerTeam))
    (if (Variables|/Game/Framework/BP_InGame_Character.BP_InGame_Character_C|GetisCarryingFlag _asbp_in_game_character)
      (CallFunction|ServerAddPoint)
      (CallFunction|ServerResetFlag _asbp_in_game_character)
      (CallFunction|ChangeState _asbp_in_game_character))
    (elif (Variables|Default|GethasFlag)
      (CallFunction|ServerPlayerPickUpFlag _asbp_in_game_character)
      (CallFunction|ChangeState _asbp_in_game_character 1))))

(event Custom|Server_ResetFlag
  (params (Player :type BP%20in%20Game%20Character%20Object%20Reference))
  (Variables|BP_FlagBase_C|SethasFlag (Variables|/Game/Framework/BP_InGame_Character.BP_InGame_Character_C|GetEnemyFlagBase Player) true)
  (Variables|/Game/Framework/BP_InGame_Character.BP_InGame_Character_C|SetisCarryingFlag Player false))

(event Custom|Server_AddPoint
  (Variables|Default|SetTeamPoints (+ (Variables|Default|GetTeamPoints) 1)))

(event Custom|Server_PlayerPickUpFlag
  (params (Player :type BP%20in%20Game%20Character%20Object%20Reference))
  (Variables|Default|SethasFlag false)
  (Variables|/Game/Framework/BP_InGame_Character.BP_InGame_Character_C|SetisCarryingFlag Player true))

(event Custom|ChangeState
  (params (Player :type BP%20in%20Game%20Character%20Object%20Reference) (0Cube1Sphere :type Integer))
  (bind _enemyflagbase (Variables|/Game/Framework/BP_InGame_Character.BP_InGame_Character_C|GetEnemyFlagBase Player))
  (bind _flagstate (Variables|BP_FlagBase_C|GetFlagState _enemyflagbase))
  (if (== 0Cube1Sphere 0)
    (if (== (Variables|/Game/Framework/BP_InGame_Character.BP_InGame_Character_C|GetTeamTag Player) "RED")
      (Components|StaticMesh|SetStaticMesh _flagstate "/Game/FirstPerson/Maps/_GENERATED/mackz/flag2.flag2")
      (else
        (Components|StaticMesh|SetStaticMesh _flagstate "/Game/FirstPerson/Maps/_GENERATED/mackz/flag.flag")))
    (else
      (Components|StaticMesh|SetStaticMesh _flagstate "/Game/FirstPerson/Maps/_GENERATED/mackz/flag1.flag1"))))

(fn ConstructionScript
  (Components|Sphere|SetSphereRadius (Variables|Default|GetRadious) (Variables|Default|GetRadiousValue) true))